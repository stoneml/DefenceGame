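; LittleMonster1_BP is the Blueprint for a small monster character, with components attached to points on its body.
; Its construction script runs the parent's, then attaches the head particle, hand, joint, fire and tail components to matching sockets on the mesh.
; Each attachment snaps to the socket location while keeping world rotation and scale.
; The event graph holds only disabled placeholder events, so it adds no gameplay logic.
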(event EventBeginPlay)

(event Collision|EventActorBeginOverlap
  (params (OtherActor :type Actor%20Object%20Reference)))

(event EventTick
  (params (DeltaSeconds :type Float%20%28single-precision%29)))

(fn ConstructionScript
  (bind _mesh (Variables|Character|GetMesh))
  (|CallParentFunction)
  (Transformation|AttachComponentToComponent (Variables|Default|GetHeadParticle) _mesh "Head" "SnapToTarget" "KeepWorld" "KeepWorld" true)
  (Transformation|AttachComponentToComponent (Variables|Default|GetL_Hand) _mesh "L_Hand" "SnapToTarget" "KeepWorld" "KeepWorld" true)
  (Transformation|AttachComponentToComponent (Variables|Default|GetR_Hand) _mesh "R_Hand" "SnapToTarget" "KeepWorld" "KeepWorld" true)
  (Transformation|AttachComponentToComponent (Variables|Default|GetL_Joint) _mesh "L_Joint" "SnapToTarget" "KeepWorld" "KeepWorld" true)
  (Transformation|AttachComponentToComponent (Variables|Default|GetR_Joint) _mesh "R_Joint" "SnapToTarget" "KeepWorld" "KeepWorld" true)
  (Transformation|AttachComponentToComponent (Variables|Default|GetFire) _mesh "Fire" "SnapToTarget" "KeepWorld" "KeepWorld" true)
  (Transformation|AttachComponentToComponent (Variables|Default|GetTail) _mesh "Tail" "SnapToTarget" "KeepWorld" "KeepWorld" true))